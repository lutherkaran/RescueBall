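; Collectible pickup that extends the countdown timer when the player touches it.
; Each tick it spins its Cylinder mesh and plays a timeline that drives the actor's scale.
; A Box overlap with PlayerBP plays a coin sound, adds time to each CountdownTimer in the player's CountdownRef array, and destroys the pickup.
; Failed casts of the player pawn or timer references print a debug message.
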(event OnComponentBeginOverlap(Box)
  (params (OtherActor :type Actor%20Object%20Reference) (OtherComp :type Primitive%20Component%20Object%20Reference) (OtherBodyIndex :type Integer) (bFromSweep :type Boolean) (SweepResult :type Hit%20Result%20Structure%20%28by%20ref%29))
  (Utilities|Casting|CastToPlayerBP OtherActor)
  (Audio|PlaySound2D "/Game/Sounds/Coin.Coin" 0.5 1.0)
  (bind _asplayer_bp (Utilities|Casting|CastToPlayerBP (Game|Player|GetPlayerPawn 0))
    (:then
      (for _array_element (Variables|/Game/Blueprints/PlayerBP.PlayerBP_C|GetcountdownRef _asplayer_bp)
        (bind _ascountdown_timer (Utilities|Casting|CastToCountdownTimer _array_element)
          (:then
            (Variables|/Script/RescueBall.CountdownTimer|SetCountdownTime _ascountdown_timer (+ (Variables|/Script/RescueBall.CountdownTimer|GetCountdownTime _ascountdown_timer) 20))
            (Actor|DestroyActor))
          (:CastFailed
            (Development|PrintString "FAILED")))))
    (:CastFailed
      (Development|PrintString "FAILED"))))

(event EventBeginPlay)

(event Collision|EventActorBeginOverlap
  (params (OtherActor :type Actor%20Object%20Reference)))

(event EventTick
  (params (DeltaSeconds :type Float%20%28single-precision%29))
  (bind _cylinder (Variables|Default|GetCylinder))
  (bind _relativerotation (Variables|/Script/Engine.SceneComponent|GetRelativeRotation _cylinder))
  (Transformation|SetRelativeRotation _cylinder (Math|Rotator|MakeRotator (+ (.roll _relativerotation) 1.0) (.pitch _relativerotation) (.yaw _relativerotation)) false false)
  (bind _scale (Timeline|ScaleTimeline Play)
    (:Update
      (Transformation|SetActorScale3D _scale))))

(fn ConstructionScript)